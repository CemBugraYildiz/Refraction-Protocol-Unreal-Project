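; BP_Indicator is an actor that shows an on or off state by changing the material on its Plane component.
; The construction script picks the initial material from the ShowFromStart flag.
; The Turn event takes an On or Off signal, swaps between the indicator and false-indicator materials, then plays a data-table sound at the actor's location.
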(event EventTurn
  (params (Signal :type Enum_Signal%20Enum :default "NewEnumerator0"))
  (bind _plane (Variables|Default|GetPlane))
  (switch Utilities|FlowControl|Switch|SwitchonEnum_Signal Signal
    (:NewEnumerator0
      (Rendering|Material|SetMaterial _plane 0 "/Game/Assets/Materials/M_Indicator.M_Indicator"))
    (:NewEnumerator1
      (Rendering|Material|SetMaterial _plane 0 "/Game/Assets/Materials/Instance/MI_IndicatorFalse.MI_IndicatorFalse")))
  (CallFunction|PlaySoundbyDataTable "BP_Indicator" (Transformation|GetActorLocation) 0.5))

(fn ConstructionScript
  (bind _plane (Variables|Default|GetPlane))
  (if (Variables|Default|GetShowFromStart)
    (Rendering|Material|SetMaterial _plane 0 "/Game/Assets/Materials/M_Indicator.M_Indicator")
    (else
      (Rendering|Material|SetMaterial _plane 0 "/Game/Assets/Materials/Instance/MI_IndicatorFalse.MI_IndicatorFalse"))))