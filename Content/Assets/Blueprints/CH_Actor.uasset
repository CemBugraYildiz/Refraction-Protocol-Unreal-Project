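; Player character Blueprint that handles sound feedback, laser-cube reflection and a few hotkeys.
; A self-looping delay plays footsteps while the character moves grounded, with intervals shrinking as speed rises.
; BeginPlay caches an attached, stopped laser sound that shoot events toggle, while standard shots play one-shot sounds.
; Laser-cube hits fetch reflection start and end vectors; T toggles tagged tutorial texts, and Enter reloads the level in the final room.
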(event Custom|SoundControl
  (params (Play%20%28if%20false,%20then%20stop%29 :type Boolean))
  (bind _sound (Variables|Default|GetSound))
  ;[0.1042 0.1042 0.1042] Sound
  ;;[1 1 1] Sound Control
  (Utilities|IsValid (Variables|Default|GetSound)
    (:Is%20Valid
      (if Play%20%28if%20false,%20then%20stop%29
        (if (not (Audio|Components|Audio|IsPlaying _sound))
          (Audio|Components|Audio|Play _sound 0.0))
        (else
          (Audio|Components|Audio|Stop _sound))))))

(event Custom|Footsteps_Init
  (bind _returnvalue (Transformation|GetVelocity))
  (bind _returnvalue_2 (Math|Vector|VectorLength _returnvalue))
  ;[1 1 1] Footsteps
  (if (and (not (AI|Components|NavMovement|IsFalling (Variables|Character|GetCharacterMovement))) (>= _returnvalue_2 1e+02)) :!label _label
    (Utilities|FlowControl|Delay (Math|Float|Lerp 0.4 0.2 (Math|Float|NormalizetoRange _returnvalue_2 0.0 1.5e+03)))
    (CallFunction|PlaySoundbyDataTable "Player_Footsteps" (Transformation|GetActorLocation) 0.75)
    (goto _label)
    (else
      (Utilities|FlowControl|Delay 0.05)
      (goto _label))))

(event EventBeginPlay
  ;[0.1042 0.1042 0.1042] Sound
  ;;[1 1 1] Sound
  (bind _returnvalue (CallFunction|PlaySoundbyDataTableAttached "ShootType_Laser" 0.7 (Variables|Default|GetCapsuleComponent) false))
  (Audio|Components|Audio|Stop _returnvalue)
  (Variables|Default|SetSound _returnvalue)
  (CallFunction|FootstepsInit) ; Init footsteps sounds
)

(event EventOnLaserSoundControl
  (params (bPlay :type Boolean))
  (CallFunction|SoundControl bPlay))

(event EventOnStandartShootSound
  (CallFunction|PlaySoundbyDataTable "ShootType_EventGun" (Transformation|GetActorLocation) 0.5))

(event EventOnLaserCubeHit
  (params (HitActor :type Actor%20Object%20Reference))
  (bind _asbp_laser_cube (Utilities|Casting|CastToBP_LaserCube HitActor))
  (Variables|Default|SetStartVec (.Start (Default|GetReflectionVector _asbp_laser_cube)))
  (Variables|Default|SetEndVec (.End (Default|GetReflectionVector _asbp_laser_cube))))

(event Input|KeyboardEvents|Enter
  (params (Key :type Key%20Structure))
  (:Pressed
    (if (Variables|Default|GetbInFinalRoom)
      (bind _returnvalue (Game|GetCurrentLevelName true))
      (Game|OpenLevel(byName) (Utilities|String|StringToName _returnvalue)))))

(event Input|KeyboardEvents|T
  (params (Key :type Key%20Structure))
  (:Pressed
    (CallFunction|ToggleTutorialTexts)))

(fn ConstructionScript)

(fn ToggleTutorialTexts
  (Variables|Default|SetTutorialTextsVisible (not (Variables|Default|GetTutorialTextsVisible)))
  (bind _outactors (Actor|GetAllActorswithTag "TutorialText"))
  (for _array_element _outactors
    (Rendering|SetActorHiddenInGame _array_element (not (not (Variables|Default|GetTutorialTextsVisible))))))